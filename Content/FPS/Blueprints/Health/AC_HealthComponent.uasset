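; AC_HealthComponent is an FPS actor component that stores and manages health within a minimum and maximum range.
; Init sets the bounds and fills health to maximum, and every change goes through SetHealth, which clamps the value.
; Damage and Heal take absolute amounts so sign cannot invert them, and HealFull heals by the maximum.
; Getters report current health, death at the minimum, and health as a clamped fraction of the maximum.
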(fn Init
  (params (New%20Min%20Health :type Float%20%28double-precision%29) (New%20Max%20Health :type Float%20%28double-precision%29))
  (Variables|HealthCOmponent|SetMinHealth New%20Min%20Health)
  (bind _output_get (Variables|HealthCOmponent|SetMaxHealth New%20Max%20Health))
  (CallFunction|SetHealth _output_get))

(fn GetHealth
  (return (Variables|HealthCOmponent|GetHealth)))

(fn SetHealth
  (params (New%20Health :type Float%20%28double-precision%29))
  (bind _output_get (Variables|HealthCOmponent|SetHealth (CallFunction|ClampHealth New%20Health)))
  (return _output_get))

(fn ClampHealth
  (params (Value :type Float%20%28double-precision%29))
  (return (Math|Float|Clamp(Float) Value (Variables|HealthCOmponent|GetMinHealth) (Variables|HealthCOmponent|GetMaxHealth))))

(fn Damage
  (params (Damage%20Amt :type Float%20%28double-precision%29))
  (CallFunction|SetHealth (- (CallFunction|GetHealth) (Math|Float|Absolute(Float) Damage%20Amt))))

(fn Heal
  (params (Heal%20Amt :type Float%20%28double-precision%29))
  (CallFunction|SetHealth (+ (CallFunction|GetHealth) (Math|Float|Absolute(Float) Heal%20Amt))))

(fn HealFull
  (CallFunction|Heal (Variables|HealthCOmponent|GetMaxHealth)))

(fn IsDead
  (return (<= (CallFunction|GetHealth) (Variables|HealthCOmponent|GetMinHealth))))

(fn GetNormalizedHealth
  (return (Math|Float|Clamp(Float) (/ (CallFunction|GetHealth) (Variables|HealthCOmponent|GetMaxHealth)))))